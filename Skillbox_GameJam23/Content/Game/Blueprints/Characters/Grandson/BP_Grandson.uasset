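; BP_Grandson is the grandson character, exposing a children route through a getter.
; ChangeState forwards a new state to the mesh's anim instance through a message call.
; A sphere overlap detects BP_StopLight and checks whether it is red, but neither that check nor the end overlap triggers anything.
; A state-change call is left disconnected, and NPCRoute returns nothing.
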(event OnComponentBeginOverlap(Sphere)
  (params (OverlappedComponent :type Primitive%20Component%20Object%20Reference) (OtherActor :type Actor%20Object%20Reference) (OtherComp :type Primitive%20Component%20Object%20Reference) (OtherBodyIndex :type Integer) (bFromSweep :type Boolean) (SweepResult :type Hit%20Result%20Structure%20%28by%20ref%29))
  (bind _asbp_stop_light (Utilities|Casting|CastToBP_StopLight OtherActor))
  (if (Variables|/Game/Game/Blueprints/Environment/Interact/BP_StopLight.BP_StopLight_C|GetIsRed _asbp_stop_light)
    _))

(event OnComponentEndOverlap(Sphere)
  (params (OverlappedComponent :type Primitive%20Component%20Object%20Reference) (OtherActor :type Actor%20Object%20Reference) (OtherComp :type Primitive%20Component%20Object%20Reference) (OtherBodyIndex :type Integer)))

(event EventChangeState
  (params (NewState :type IE_State%20Enum :default "NewEnumerator0"))
  (Class|BPIAIHelper|ChangeState(Message) (Components|SkeletalMesh|GetAnimInstance (Variables|Character|GetMesh)) NewState))

(fn ConstructionScript)

(fn ChildrenRoute
  (return (Variables|Default|GetChildren%20Route)))

(fn NPCRoute
  (return 0))