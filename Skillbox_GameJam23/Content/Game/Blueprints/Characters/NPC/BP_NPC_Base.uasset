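; BP_NPC_Base is the base NPC character Blueprint, providing shared appearance, movement speed, animation state and route access.
; On BeginPlay it applies its walk speed to CharacterMovement and picks a random skeletal mesh from MESHES for visual variety.
; ChangeState forwards the new state to the mesh's anim instance as a message.
; NPCRoute returns the stored UsedNPCRoute, while ChildrenRoute is an empty stub.
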(event EventChangeState
  (params (NewState :type IE_State%20Enum :default "NewEnumerator0"))
  (Class|BPIAIHelper|ChangeState(Message) (Components|SkeletalMesh|GetAnimInstance (Variables|Character|GetMesh)) NewState))

(event EventBeginPlay
  (Variables|/Script/Engine.CharacterMovementComponent|SetMaxWalkSpeed (Variables|Character|GetCharacterMovement) (Variables|Default|GetMaxWalkSpeed))
  (Components|SkeletalMesh|SetSkeletalMeshAsset (Variables|Character|GetMesh) (.OutItem (Utilities|Array|Random (Variables|Default|GetMESHES)))))

(fn ConstructionScript)

(fn ChildrenRoute
  (return 0))

(fn NPCRoute
  (return (Variables|Default|GetUsedNPCRoute)))