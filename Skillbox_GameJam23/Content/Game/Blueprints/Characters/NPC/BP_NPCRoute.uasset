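; BP_NPCRoute is a patrol route for NPCs, defined by the PointRoute spline and a current point index.
; GetNextPointPosition returns the world location of the spline point at that index.
; IncrementPoint advances the index, wrapping it with a modulo on the spline's point count so the route loops.
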(event Custom|IncrementPoint
  (bind _result (Math|Integer|IncrementInt (Variables|Default|GetPointIndex))
    (:%20%20
      (Variables|Default|SetPointIndex (Math|Integer|%(Integer) _result (Spline|GetNumberOfSplinePoints (Variables|Default|GetPointRoute)))))))

(fn ConstructionScript)

(fn GetNextPointPosition
  (return (Spline|GetLocationatSplinePoint (Variables|Default|GetPointRoute) (Variables|Default|GetPointIndex) "World")))