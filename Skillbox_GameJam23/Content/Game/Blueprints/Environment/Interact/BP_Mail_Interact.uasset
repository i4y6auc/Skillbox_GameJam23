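; Mail interaction actor that lets the Granny player complete the send-letter task during a midday window of the in-game clock.
; Its trigger overlap toggles input and an interaction prompt widget, whose text is set on BeginPlay.
; On interact within hours, it sets the player's task flag, fills the progress bar and destroys itself after a delay.
; Outside hours, it briefly shows a come-back-later widget.
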(event OnComponentBeginOverlap(TriggerCollision)
  (params (OverlappedComponent :type Primitive%20Component%20Object%20Reference) (OtherActor :type Actor%20Object%20Reference) (OtherComp :type Primitive%20Component%20Object%20Reference) (OtherBodyIndex :type Integer) (bFromSweep :type Boolean) (SweepResult :type Hit%20Result%20Structure%20%28by%20ref%29))
  (if (== OtherActor (Variables|Default|GetPlayerRef))
    (Input|EnableInput (Game|GetPlayerController 0))
    (Development|SetHiddeninGame (Variables|Default|GetInteractionWidget) false false)))

(event OnComponentEndOverlap(TriggerCollision)
  (params (OverlappedComponent :type Primitive%20Component%20Object%20Reference) (OtherActor :type Actor%20Object%20Reference) (OtherComp :type Primitive%20Component%20Object%20Reference) (OtherBodyIndex :type Integer))
  (Input|DisableInput (Game|GetPlayerController 0))
  (Development|SetHiddeninGame (Variables|Default|GetInteractionWidget) true false))

(event Input|EnhancedActionEvents|EnhancedInputActionIA_Interact
  (params (ActionValue :type Boolean) (ElapsedSeconds :type Float%20%28double-precision%29) (TriggeredSeconds :type Float%20%28double-precision%29) (InputAction :type Input%20Action%20Object%20Reference :default "/Game/Game/Input/IA_Interact.IA_Interact"))
  (bind _playerref (Variables|Default|GetPlayerRef))
  (bind _playerref_2 (Variables|Default|GetPlayerRef))
  (bind _babka_time (Variables|/Game/Game/Blueprints/Player/BP_Player_Granny.BP_Player_Granny_C|GetBabka%20Time _playerref_2))
  (:Completed
    (if (and (>= _babka_time (Math|Timespan|MakeTimespan 0 11 0 0 0)) (<= _babka_time (Math|Timespan|MakeTimespan 0 15 0 0 0)))
      (Variables|/Game/Game/Blueprints/Player/BP_Player_Granny.BP_Player_Granny_C|SetTask_SendLetter _playerref true)
      (Default|FillProgressBar _playerref)
      (Utilities|FlowControl|Delay 1e+01)
      (Actor|DestroyActor)
      (else
        (bind _returnvalue (UserInterface|CreateWidget "/Game/Game/UI/WBP_MailComeBackLater.WBP_MailComeBackLater_C"))
        (UserInterface|Viewport|AddtoViewport _returnvalue 0)
        (Utilities|FlowControl|Delay 5.0)
        (Widget|RemovefromParent _returnvalue)))))

(event EventBeginPlay
  (bind _asbp_player_granny (Utilities|Casting|CastToBP_Player_Granny (Game|GetPlayerCharacter 0)))
  (Variables|Default|SetPlayerRef _asbp_player_granny)
  (bind _aswbp_interact (Utilities|Casting|CastToWBP_Interact (UserInterface|GetWidget (Variables|Default|GetInteractionWidget))))
  (Default|SetText _aswbp_interact (Variables|Default|GetInteractText)))

(fn ConstructionScript)