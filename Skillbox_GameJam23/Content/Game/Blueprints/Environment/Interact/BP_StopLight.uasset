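; Traffic stop light actor that alternates between red and green on a fixed interval.
; A looping timer started on BeginPlay flips IsRed every ChangeTime seconds, then calls SetLightVisibility.
; That function shows the matching set of four red or green components and enables the box collision only while red.
; The initial state is not applied at BeginPlay, so visibility and collision first update when the timer fires.
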(event Custom|SetLight
  (if (Variables|Default|GetIsRed)
    (Variables|Default|SetIsRed false)
    (else
      (Variables|Default|SetIsRed true)))
  (CallFunction|SetLightVisibility))

(event EventBeginPlay
  (Utilities|Time|SetTimerbyEvent (delegate Custom|SetLight) (Variables|Default|GetChangeTime) true))

(fn ConstructionScript)

(fn SetLightVisibility
  (bind _boxcollision (Variables|Default|GetBoxCollision))
  (bind _isred (Variables|Default|GetIsRed))
  (bind _returnvalue (not _isred))
  (if _isred
    (Collision|SetCollisionEnabled _boxcollision "QueryAndPhysics")
    (else
      (Collision|SetCollisionEnabled _boxcollision "NoCollision")))
  (Rendering|SetVisibility (Variables|Default|GetRed_1) _isred false)
  (Rendering|SetVisibility (Variables|Default|GetRed_2) _isred false)
  (Rendering|SetVisibility (Variables|Default|GetRed_3) _isred false)
  (Rendering|SetVisibility (Variables|Default|GetRed_4) _isred false)
  (Rendering|SetVisibility (Variables|Default|GetGreen_1) _returnvalue false)
  (Rendering|SetVisibility (Variables|Default|GetGreen_2) _returnvalue false)
  (Rendering|SetVisibility (Variables|Default|GetGreen_3) _returnvalue false)
  (Rendering|SetVisibility (Variables|Default|GetGreen_4) _returnvalue false))