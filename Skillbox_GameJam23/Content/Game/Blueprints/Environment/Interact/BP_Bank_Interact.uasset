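; BP_Bank_Interact is a bank interactable where the granny player collects money, usable only during a morning window of in-game time.
; A trigger shows the prompt widget and enables input for IA_Interact.
; The first interaction sets a ready time 40 game minutes later and shows a "come back later" widget; early retries show another.
; Once ready, GiveMoney fills the player's progress bar, flags the task, adds money and destroys the actor.
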(event OnComponentBeginOverlap(TriggerCollision)
  (params (OverlappedComponent :type Primitive%20Component%20Object%20Reference) (OtherActor :type Actor%20Object%20Reference) (OtherComp :type Primitive%20Component%20Object%20Reference) (OtherBodyIndex :type Integer) (bFromSweep :type Boolean) (SweepResult :type Hit%20Result%20Structure%20%28by%20ref%29))
  (Input|EnableInput (Game|GetPlayerController 0))
  (Development|SetHiddeninGame (Variables|Default|GetInteractionWidget) false false))

(event OnComponentEndOverlap(TriggerCollision)
  (params (OverlappedComponent :type Primitive%20Component%20Object%20Reference) (OtherActor :type Actor%20Object%20Reference) (OtherComp :type Primitive%20Component%20Object%20Reference) (OtherBodyIndex :type Integer))
  (Input|DisableInput (Game|GetPlayerController 0))
  (Development|SetHiddeninGame (Variables|Default|GetInteractionWidget) true false))

(event Input|EnhancedActionEvents|EnhancedInputActionIA_Interact
  (params (ActionValue :type Boolean) (ElapsedSeconds :type Float%20%28double-precision%29) (TriggeredSeconds :type Float%20%28double-precision%29) (InputAction :type Input%20Action%20Object%20Reference :default "/Game/Game/Input/IA_Interact.IA_Interact"))
  (bind _playerref (Variables|Default|GetPlayerRef))
  (bind _babka_time (Variables|/Game/Game/Blueprints/Player/BP_Player_Granny.BP_Player_Granny_C|GetBabka%20Time _playerref))
  (:Completed
    (if (and (>= _babka_time (Math|Timespan|MakeTimespan 0 9 0 0 0)) (<= _babka_time (Math|Timespan|MakeTimespan 0 12 0 0 0)))
      (Variables|Default|SetCurrentTime (Variables|/Game/Game/Blueprints/Player/BP_Player_Granny.BP_Player_Granny_C|GetBabka%20Time (Variables|Default|GetPlayerRef)))
      (if (Variables|Default|GetIsFirstTry)
        (Variables|Default|SetIsFirstTry false)
        (Variables|Default|SetNeedTime (+ (Variables|Default|GetCurrentTime) (Math|Timespan|MakeTimespan 0 0 40 0 0)))
        (bind _returnvalue (UserInterface|CreateWidget "/Game/Game/UI/WBP_MailComeBackLater.WBP_MailComeBackLater_C"))
        (UserInterface|Viewport|AddtoViewport _returnvalue 0)
        (Variables|Default|SetSeeFirstWidget true)
        (Utilities|FlowControl|Delay 5.0)
        (Widget|RemovefromParent _returnvalue)
        (Variables|Default|SetSeeFirstWidget false)
        (elif (>= (Variables|Default|GetCurrentTime) (Variables|Default|GetNeedTime))
          (CallFunction|GiveMoney)
          (elif (not (Variables|Default|GetSeeFirstWidget))
            (Utilities|FlowControl|DoOnce false :!label _label
              (:Completed
                (bind _returnvalue_2 (UserInterface|CreateWidget "/Game/Game/UI/WBP_MailComeBackLater.WBP_MailComeBackLater_C"))
                (UserInterface|Viewport|AddtoViewport _returnvalue_2 0)
                (Rendering|Components|TextRender|SetText (Variables|/Game/Game/UI/WBP_MailComeBackLater.WBP_MailComeBackLater_C|GetTextLeter _returnvalue_2) (Variables|Default|GetTextLeter))
                (Utilities|FlowControl|Delay 5.0)
                (Widget|RemovefromParent _returnvalue_2)
                (goto _label Reset)))))))))

(event EventBeginPlay
  (bind _asbp_player_granny (Utilities|Casting|CastToBP_Player_Granny (Game|GetPlayerCharacter 0)))
  (Variables|Default|SetPlayerRef _asbp_player_granny)
  (Variables|Default|SetIsFirstTry true)
  (bind _aswbp_interact (Utilities|Casting|CastToWBP_Interact (UserInterface|GetWidget (Variables|Default|GetInteractionWidget))))
  (Default|SetText _aswbp_interact (Variables|Default|GetInteractText)))

(fn ConstructionScript)

(fn GiveMoney
  (bind _playerref (Variables|Default|GetPlayerRef))
  (Default|FillProgressBar _playerref)
  (Variables|/Game/Game/Blueprints/Player/BP_Player_Granny.BP_Player_Granny_C|SetTask_GetMoney _playerref true)
  (Variables|/Game/Game/Blueprints/Player/BP_Player_Granny.BP_Player_Granny_C|SetMoney _playerref (+ (Variables|/Game/Game/Blueprints/Player/BP_Player_Granny.BP_Player_Granny_C|GetMoney _playerref) (Variables|Default|GetAddMoney)))
  (Actor|DestroyActor))