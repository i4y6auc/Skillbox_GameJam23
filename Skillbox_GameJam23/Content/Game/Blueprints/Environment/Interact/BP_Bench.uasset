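; Interactable bench that lets the granny player sit, doubling BaseResPressure until they get up.
; Trigger overlap enables input and shows a prompt widget; IA_Interact alternates between sitting and standing through a FlipFlop.
; Sitting fakes the pose by hiding and freezing the player, showing the bench's own skeletal mesh and blending to the bench camera; standing reverses this.
; The bench mesh comes from CurrentBench at BeginPlay, and the black-screen popup logic is unconnected.
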(event OnComponentBeginOverlap(TriggerCollision)
  (params (OverlappedComponent :type Primitive%20Component%20Object%20Reference) (OtherActor :type Actor%20Object%20Reference) (OtherComp :type Primitive%20Component%20Object%20Reference) (OtherBodyIndex :type Integer) (bFromSweep :type Boolean) (SweepResult :type Hit%20Result%20Structure%20%28by%20ref%29))
  (if (== OtherActor (Variables|Default|GetPlayerRef))
    (Input|EnableInput (Game|GetPlayerController 0))
    (Development|SetHiddeninGame (Variables|Default|GetInteractionWidget) false false)
    (Variables|Default|SetCameraOwner (Components|GetOwner (Variables|Default|GetCamera)))))

(event OnComponentEndOverlap(TriggerCollision)
  (params (OverlappedComponent :type Primitive%20Component%20Object%20Reference) (OtherActor :type Actor%20Object%20Reference) (OtherComp :type Primitive%20Component%20Object%20Reference) (OtherBodyIndex :type Integer))
  (if (== OtherActor (Variables|Default|GetPlayerRef))
    (Input|DisableInput (Game|GetPlayerController 0))
    (Development|SetHiddeninGame (Variables|Default|GetInteractionWidget) true false)))

(event Input|EnhancedActionEvents|EnhancedInputActionIA_Interact
  (params (ActionValue :type Boolean) (ElapsedSeconds :type Float%20%28double-precision%29) (TriggeredSeconds :type Float%20%28double-precision%29) (InputAction :type Input%20Action%20Object%20Reference :default "/Game/Game/Input/IA_Interact.IA_Interact"))
  (bind _returnvalue (Game|GetPlayerController 0))
  (bind _widgetref (Variables|Default|GetWidgetRef))
  (bind _playerref (Variables|Default|GetPlayerRef))
  (bind _playerref_2 (Variables|Default|GetPlayerRef))
  (bind _playerref_3 (Variables|Default|GetPlayerRef))
  (bind _skeletalmesh (Variables|Default|GetSkeletalMesh))
  (bind _playerref_4 (Variables|Default|GetPlayerRef))
  (bind _charactermovement (Variables|/Script/Engine.Character|GetCharacterMovement _playerref_4))
  (:Completed
    (Utilities|FlowControl|FlipFlop
      (:A
        (Pawn|Components|CharacterMovement|DisableMovement _charactermovement)
        (Rendering|SetActorHiddenInGame _playerref_3 true)
        (Development|SetHiddeninGame _skeletalmesh false false)
        (Game|Player|SetViewTargetwithBlend _returnvalue (Variables|Default|GetCameraOwner) 0.8 "VTBlend_Linear" 0.0 false)
        (Default|SetText _widgetref (Variables|Default|GetDeactivateText))
        (Variables|/Game/Game/Blueprints/Player/BP_Player_Granny.BP_Player_Granny_C|SetBaseResPressure _playerref_2 (* (Variables|/Game/Game/Blueprints/Player/BP_Player_Granny.BP_Player_Granny_C|GetBaseResPressure _playerref_2) 2)))
      (:B
        (Pawn|Components|CharacterMovement|SetMovementMode _charactermovement "MOVE_Walking" 0)
        (Rendering|SetActorHiddenInGame _playerref_3 false)
        (Development|SetHiddeninGame _skeletalmesh true false)
        (Game|Player|SetViewTargetwithBlend _returnvalue (Components|GetOwner (Variables|/Game/Game/Blueprints/Player/BP_Player_Granny.BP_Player_Granny_C|GetCamera (Variables|Default|GetPlayerRef))) 0.8 "VTBlend_Linear" 0.0 false)
        (Default|SetText _widgetref (Variables|Default|GetActivateText))
        (Variables|/Game/Game/Blueprints/Player/BP_Player_Granny.BP_Player_Granny_C|SetBaseResPressure _playerref (/ (Variables|/Game/Game/Blueprints/Player/BP_Player_Granny.BP_Player_Granny_C|GetBaseResPressure _playerref) 2))))))

(event EventBeginPlay
  (bind _currentbench (Variables|Default|GetCurrentBench))
  (bind _asbp_player_granny (Utilities|Casting|CastToBP_Player_Granny (Game|GetPlayerCharacter 0)))
  (Variables|Default|SetPlayerRef _asbp_player_granny)
  (Utilities|IsValid _currentbench
    (:Is%20Valid
      (Components|StaticMesh|SetStaticMesh (Variables|Default|GetSM_Bench) _currentbench)
      (bind _aswbp_interact (Utilities|Casting|CastToWBP_Interact (UserInterface|GetWidget (Variables|Default|GetInteractionWidget))))
      (bind _output_get (Variables|Default|SetWidgetRef _aswbp_interact))
      (Default|SetText _output_get (Variables|Default|GetActivateText)))))

(fn ConstructionScript)

(fn NewFunction
  (params (self2 :type Actor%20Object%20Reference)))

(fn BlackScreenPop)