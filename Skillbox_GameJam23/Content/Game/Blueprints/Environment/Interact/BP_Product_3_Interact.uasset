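; BP_Product_3_Interact is an environment interactable for the granny player's task of buying product 3.
; On BeginPlay it caches the player character as BP_Player_Granny.
; Overlapping its trigger enables input on the actor and shows an interaction widget, and leaving reverses both.
; Completing IA_Interact sets the player's TaskBuyProduct3 flag and calls FillProgressBar on the player.
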(event OnComponentBeginOverlap(TriggerCollision)
  (params (OverlappedComponent :type Primitive%20Component%20Object%20Reference) (OtherActor :type Actor%20Object%20Reference) (OtherComp :type Primitive%20Component%20Object%20Reference) (OtherBodyIndex :type Integer) (bFromSweep :type Boolean) (SweepResult :type Hit%20Result%20Structure%20%28by%20ref%29))
  (Input|EnableInput (Game|GetPlayerController 0))
  (Development|SetHiddeninGame (Variables|Default|GetInteractionWidget) false false))

(event OnComponentEndOverlap(TriggerCollision)
  (params (OverlappedComponent :type Primitive%20Component%20Object%20Reference) (OtherActor :type Actor%20Object%20Reference) (OtherComp :type Primitive%20Component%20Object%20Reference) (OtherBodyIndex :type Integer))
  (Input|DisableInput (Game|GetPlayerController 0))
  (Development|SetHiddeninGame (Variables|Default|GetInteractionWidget) true false))

(event Input|EnhancedActionEvents|EnhancedInputActionIA_Interact
  (params (ActionValue :type Boolean) (ElapsedSeconds :type Float%20%28double-precision%29) (TriggeredSeconds :type Float%20%28double-precision%29) (InputAction :type Input%20Action%20Object%20Reference :default "/Game/Game/Input/IA_Interact.IA_Interact"))
  (bind _playerref (Variables|Default|GetPlayerRef))
  (:Completed
    (Variables|/Game/Game/Blueprints/Player/BP_Player_Granny.BP_Player_Granny_C|SetTask_Buy_Product_3 _playerref true)
    (Default|FillProgressBar _playerref)))

(event EventBeginPlay
  (bind _asbp_player_granny (Utilities|Casting|CastToBP_Player_Granny (Game|GetPlayerCharacter 0)))
  (Variables|Default|SetPlayerRef _asbp_player_granny))

(fn ConstructionScript)