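; BP_NPCRoute is a patrol route for an NPC, filed under the Grandson AI, that defines waypoints as points on the PointRoute spline.
; GetNextPointPosition returns the world location of the spline point at the current PointIndex.
; IncrementPoint advances that index and wraps it by the spline's point count, so the route loops.
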(event Custom|IncrementPoint
  (bind _result (Math|Integer|IncrementInt (Variables|Default|GetPointIndex))
    (:%20%20
      (Variables|Default|SetPointIndex (Math|Integer|%(Integer) _result (Spline|GetNumberOfSplinePoints (Variables|Default|GetPointRoute)))))))

(event EventBeginPlay)

(event Collision|EventActorBeginOverlap
  (params (OtherActor :type Actor%20Object%20Reference)))

(event EventTick
  (params (DeltaSeconds :type Float%20%28single-precision%29)))

(fn ConstructionScript)

(fn GetNextPointPosition
  (return (Spline|GetLocationatSplinePoint (Variables|Default|GetPointRoute) (Variables|Default|GetPointIndex) "World")))